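; Player controller for a networked test game, handling pawn movement, rolling, camera look and text chat.
; Move axes and Roll go through server events to multicast events on the controlled BP_TestPawn, replicating input to every copy.
; Enter focuses the HUD chat; Server_SendMessage has the cached game mode broadcast messages, and SendMessageToHUD passes them to the HUD widget.
; Mouse axes add yaw and pitch locally.
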(event Custom|SendMessageToHUD
  (params (Sender :type String) (Message :type String))
  ;[0.8145 0.8398 1] Логика отправления сообщения из чата
  ;;[1 1 1] Передаём своему HUD данные для дальнейших манипуляций
  (bind _asbp_net_test_hud (Utilities|Casting|CastToBP_NetTestHUD (HUD|GetHUD)))
  (Default|SendMessagetoWidget _asbp_net_test_hud Sender Message))

(event Custom|Server_SendMessage
  (params (Sender :type String) (Message :type String))
  ;[0.8145 0.8398 1] Логика отправления сообщения из чата
  ;;[1 1 1] Отправляем данные на сервер
  (Default|SendMessagetoEveryone (Variables|Default|GetNetTestGamemode) Sender Message))

(event Custom|Server_PlayMontage
  ;[1 0.6919 0.642] Логика игрового кувырка в PlayerController'е
  ;;[1 1 1] Вызываем на сервере событие Pawn'а
  (bind _asbp_test_pawn (Utilities|Casting|CastToBP_TestPawn (Pawn|GetControlledPawn)))
  (Default|MulticastStartRoll _asbp_test_pawn))

(event Custom|Server_MoveRight
  (params (AxisValue :type Float%20%28single-precision%29))
  ;[1 0.6235 0.6036] Настройки управления
  ;;[1 1 1] Отправляем на сервер данные нажатых клавиш чтобы задать управления всем свои копиям на всех мирах
  (bind _asbp_test_pawn (Utilities|Casting|CastToBP_TestPawn (Pawn|GetControlledPawn)))
  (Default|MulticastMoveRight _asbp_test_pawn AxisValue))

(event Custom|Server_MoveForward
  (params (AxisValue :type Float%20%28single-precision%29))
  ;[1 0.6235 0.6036] Настройки управления
  ;;[1 1 1] Отправляем на сервер данные нажатых клавиш чтобы задать управления всем свои копиям на всех мирах
  (bind _asbp_test_pawn (Utilities|Casting|CastToBP_TestPawn (Pawn|GetControlledPawn)))
  (Default|MulticastMoveForward _asbp_test_pawn AxisValue))

(event EventBeginPlay
  ;[1 0.6573 0.5873] Сохраняем ссылку на Gamemode
  (bind _asbp_net_test_gamemode (Utilities|Casting|CastToBP_NetTestGameMode (Game|GetGameMode)))
  (Variables|Default|SetNetTestGamemode _asbp_net_test_gamemode))

(event Input|ActionEvents|InputActionRoll
  (params (Key :type Key%20Structure))
  ;[1 0.6919 0.642] Логика игрового кувырка в PlayerController'е
  ;;[1 1 1] Вызываем на сервере событие Pawn'а
  (:Pressed
    (CallFunction|ServerPlayMontage)))

(event Input|AxisEvents|InputAxisMoveRight
  (params (AxisValue :type Float%20%28single-precision%29))
  ;[1 0.6235 0.6036] Настройки управления
  ;;[1 1 1] Отправляем на сервер данные нажатых клавиш чтобы задать управления всем свои копиям на всех мирах
  (CallFunction|ServerMoveRight AxisValue))

(event Input|AxisEvents|InputAxisMoveForward
  (params (AxisValue :type Float%20%28single-precision%29))
  ;[1 0.6235 0.6036] Настройки управления
  ;;[1 1 1] Отправляем на сервер данные нажатых клавиш чтобы задать управления всем свои копиям на всех мирах
  (CallFunction|ServerMoveForward AxisValue))

(event Input|AxisEvents|InputAxisMouseHorizontal
  (params (AxisValue :type Float%20%28single-precision%29))
  ;[1 0.6235 0.6036] Настройки управления
  ;;[1 1 1] Управление камерой
  (Class|PlayerController|AddYawInput AxisValue))

(event Input|AxisEvents|InputAxisMouseVertical
  (params (AxisValue :type Float%20%28single-precision%29))
  ;[1 0.6235 0.6036] Настройки управления
  ;;[1 1 1] Управление камерой
  (Class|PlayerController|AddPitchInput AxisValue))

(event Input|KeyboardEvents|Enter
  (params (Key :type Key%20Structure))
  ;[0.8145 0.8398 1] Логика отправления сообщения из чата
  ;;[1 1 1] Активируем чат
  (:Pressed
    (bind _asbp_net_test_hud (Utilities|Casting|CastToBP_NetTestHUD (HUD|GetHUD)))
    (Default|FocusChat _asbp_net_test_hud)))

(fn ConstructionScript)