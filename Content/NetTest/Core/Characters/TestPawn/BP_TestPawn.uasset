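; BP_TestPawn is a network test character with multicast forward/right movement and a timed roll.
; The roll async-loads and plays a montage on each copy while disabling input on the cached player-0 BP_NetTestPlayerController.
; During the roll, Tick pushes the character forward, setting MaxWalkSpeed from a curve over RollDuration.
; A temporarily raised MaxAcceleration makes speed follow the curve almost instantly, and is restored afterward.
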(event Custom|Multicast_StartRoll
  (bind _charactermovement (Variables|Character|GetCharacterMovement))
  (bind _testplayercontroller (Variables|Default|GetTestPlayerController))
  (bind _testplayercontroller_2 (Variables|Default|GetTestPlayerController))
  ;[1 1 1] Проигрываем монтаж на всех своих копиях во всех мирах и в конце обнуляем таймер
  (Variables|Default|SetbRoll true)
  (Variables|Default|SetDefaultMaxAcceleration (Class|CharacterMovementComponent|GetMaxAcceleration _charactermovement))
  (Variables|/Script/Engine.CharacterMovementComponent|SetMaxAcceleration _charactermovement 7e+03)
  (bind _object (Utilities|AsyncLoadAsset (Variables|Default|GetRollMontage))
    (:Completed
      (Input|DisableInput _testplayercontroller_2 _testplayercontroller_2)
      (Animation|PlayAnimMontage (.AsAnim%20Montage (Utilities|Casting|CastToAnimMontage _object)) 1.0 "None")
      (Utilities|FlowControl|Delay (Variables|Default|GetRollDuration))
      (Variables|Default|SetbRoll false)
      (Variables|Default|SetTimer 0.0)
      (Variables|/Script/Engine.CharacterMovementComponent|SetMaxAcceleration (Variables|Character|GetCharacterMovement) (Variables|Default|GetDefaultMaxAcceleration))
      (Input|EnableInput _testplayercontroller _testplayercontroller))))

(event Custom|Multicast_MoveRight
  (params (AxisValue :type Float%20%28single-precision%29))
  ;[1 1 1] Настройка движения вперёд-назад
  ;;[1 1 1] Задаём движение всем нашим копиям во всех мирах
  (Pawn|Input|AddMovementInput (Transformation|GetActorRightVector) AxisValue false))

(event Custom|Multicast_MoveForward
  (params (AxisValue :type Float%20%28single-precision%29))
  ;[1 1 1] Настройка движения вперёд-назад
  ;;[1 1 1] Задаём движение всем нашим копиям во всех мирах
  (Pawn|Input|AddMovementInput (Transformation|GetActorForwardVector) AxisValue false))

(event EventBeginPlay
  (bind _asbp_net_test_player_controller (Utilities|Casting|CastToBP_NetTestPlayerController (Game|GetPlayerController 0)))
  (Variables|Default|SetTestPlayerController _asbp_net_test_player_controller))

(event EventTick
  (params (DeltaSeconds :type Float%20%28single-precision%29))
  (if (Variables|Default|GetbRoll)
    (Variables|Default|SetTimer (+ DeltaSeconds (Variables|Default|GetTimer)))
    ;[1 1 1] Говорим персонажу идти вперед. Персонаж всегда будет двигаться со скоростью MaxWalkSpeed, потому что мы выставили относительно большой MaxAcceleration, чтобы персонаж почти мгновенно набирал свою максимальную скорость. Значения MaxWalkSpeed указываются в кривой
    (Variables|/Script/Engine.CharacterMovementComponent|SetMaxWalkSpeed (Variables|Character|GetCharacterMovement) (Math|Curves|GetFloatValue (Variables|Default|GetCurveFloat) (/ (Variables|Default|GetTimer) (Variables|Default|GetRollDuration))))
    (Pawn|Input|AddMovementInput (Transformation|GetActorForwardVector) 1.0 false)))

(fn ConstructionScript)